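; BP_Zerczak is a creature actor driven by Health, Experience and ChargeAttack components.
; Charge hits deal point damage, injuries grow its scale up to a clamp, and leveling up heals it by its max health.
; On death it grants its current experience to the killer and destroys itself, but only if that killer has an ExperienceComponent.
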(event `self.Health.onDeath`
  (params (deathCauser :type "Actor Object Reference"))
  (bind _returnvalue (`self.GetComponentByClass` deathCauser "/Script/Beetrayal.ExperienceComponent"))
  (if (`KismetSystemLibrary.IsValid` deathCauser)
    (if (`KismetSystemLibrary.IsValid` _returnvalue)
      (`ExperienceComponent.gain_experience` _returnvalue (`ExperienceComponent.get_current_experience` (`self.Experience`)))
      (`self.K2_DestroyActor`))))

(event `self.Health.onInjure`
  (params (deathCauser :type "Actor Object Reference"))
  (`KismetSystemLibrary.PrintString` "OUGH")
  (`self.SetActorScale3D` (`KismetMathLibrary.ClampVectorSize` (* (`self.GetActorScale3D`) 1.1) 0.1 8.0)))

(event `self.ChargeAttack.onChargeHit`
  (params (otherActor :type "Actor Object Reference") (hitInfo :type "HitResult Structure (by ref)"))
  (`GameplayStatics.ApplyPointDamage` otherActor 30.0 (`self.K2_GetActorLocation`) hitInfo (`self.GetController` self) self))

(event `self.Experience.onLevelUp`
  (bind _returnvalue (`HealthComponent.get_max_health` (`self.Health`)))
  (`HealthComponent.heal` (`self.Health`) _returnvalue null)
  (`KismetSystemLibrary.PrintString` "Zerczak level UP"))

(fn `UserConstructionScript`)