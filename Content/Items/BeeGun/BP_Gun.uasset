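; BP_Gun is a pickup gun weapon that attaches to the character who picks it up, shutting off its Niagara effect and, on successful attach, its collision and animation.
; Its Weapon component drives combat through events, with each attack reporting a noise event at the instigator's location.
; Each hit applies point damage, pushes physics-simulating components along the trace direction, and adds a radial impulse to Geometry Collections at the impact point.
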(event `self.ReceiveBeginPlay`)

(event `self.pick`
  (params (character :type "Rubee Object Reference"))
  (`ActorComponent.Deactivate` (`self.Niagara`))
  (bind _returnvalue (`WeaponComponent.attach` (`self.Weapon`) character))
  (if _returnvalue
    (`self.SetActorEnableCollision` false)
    (`self.set_animated` false)))

(event `self.Weapon.onAttack`
  (params (instigator :type "Character Object Reference"))
  (`AISense_Hearing.ReportNoiseEvent` (`self.K2_GetActorLocation` instigator) 100.0 instigator))

(event `self.Weapon.OnComponentHit`
  (params (HitComponent :type "PrimitiveComponent Object Reference") (OtherActor :type "Actor Object Reference") (OtherComp :type "PrimitiveComponent Object Reference") (NormalImpulse :type "Vector Structure") (Hit :type "HitResult Structure (by ref)"))
  (`|ExecutionSequence`
    (:`then_0`
      (bind _output_get (set `self.Hit` Hit))
      (if (`SceneComponent.IsSimulatingPhysics` OtherComp "None")
        (bind _returnvalue (- (`.TraceEnd` (`GameplayStatics.BreakHitResult` _output_get)) (`.TraceStart` (`GameplayStatics.BreakHitResult` _output_get))))
        (`PrimitiveComponent.AddImpulseAtLocation` OtherComp (* _returnvalue 10.0) (`.Location` (`GameplayStatics.BreakHitResult` _output_get)) (`.BoneName` (`GameplayStatics.BreakHitResult` _output_get)))))
    (:`then_1`
      (`GameplayStatics.ApplyPointDamage` OtherActor 10.0 _returnvalue Hit))
    (:`then_2`
      (bind _asgeometry_collection_component (cast `GeometryCollectionComponent` OtherComp))
      (`PhysicsObjectBlueprintLibrary.ApplyRadialImpulse` _asgeometry_collection_component (`.ImpactPoint` (`GameplayStatics.BreakHitResult` _output_get)) 20.0 1000.0 "RIF_Constant"))))

(fn `UserConstructionScript`)