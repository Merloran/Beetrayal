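; BP_Pot is a breakable pot interactive object that spawns an item when it shatters.
; Its Geometry Collection's Chaos break event, ignoring breaks with index 1, switches the collection's collision object type to a custom channel.
; It then calls SpawnItem on an ItemSpawner held in a child actor component, with a HasSpawned flag limiting the spawn to once.
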(event `self.GeometryCollection.OnChaosBreakEvent`
  (params (BreakEvent :type "ChaosBreakEvent Structure (by ref)"))
  ;[1 1 1] Technological debt ;p
  (if (!= BreakEvent_Index 1)
    (`PrimitiveComponent.SetCollisionObjectType` (`self.GeometryCollection`) "ECC_GameTraceChannel1")
    (if (not (`self.hasSpawned`))
      (bind _asitem_spawner (cast `ItemSpawner` (`ChildActorComponent.ChildActor` (`self.BP_ItemSpawner`)))
        (:`then`
          (`ItemSpawner.spawn_item` _asitem_spawner)
          (set `self.hasSpawned` true))
        (:`CastFailed`
          (`KismetSystemLibrary.PrintString` "Hello"))))))

(fn `UserConstructionScript`)