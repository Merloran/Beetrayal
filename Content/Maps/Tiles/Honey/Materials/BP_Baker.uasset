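; BP_Baker is an editor-time helper actor that bakes a material into a static texture, stored among the Honey tile map materials.
; Its Bake function clears a render target to black, draws the material into it, then saves the result as TEX_HEX with normal map compression.
; The bake runs only when both the material and render target are valid, and the texture creation step is editor-only.
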(fn `Bake`
  (if (and (`KismetSystemLibrary.IsValid` (`self.Material`)) (`KismetSystemLibrary.IsValid` (`self.RenderTarget`)))
    (`KismetRenderingLibrary.ClearRenderTarget2D` (`self.RenderTarget`))
    (`KismetRenderingLibrary.DrawMaterialToRenderTarget` (`self.RenderTarget`) (`self.Material`))
    (`KismetRenderingLibrary.RenderTargetCreateStaticTexture2DEditorOnly` (`self.RenderTarget`) "TEX_HEX" "TC_Normalmap")))

(fn `UserConstructionScript`)